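; A switch-driven door built from six AnimatedCube child actors that animate at individual speeds.
; The construction script gathers the child actor components and fills their play rates with either a fixed preset or, with RandomSpeed, clamped random values.
; SwitchSignal re-rolls the rates when RandomSpeed is on, then applies each to its cube's MoveTimeline and forwards the on/off signal.
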(event EventBeginPlay)

(event Collision|EventActorBeginOverlap
  (params (OtherActor :type Actor%20Object%20Reference)))

(event EventTick
  (params (DeltaSeconds :type Float%20%28single-precision%29)))

(event EventSwitchSignal
  (params (SignalOnOff :type Boolean))
  (if (Variables|Default|GetRandomSpeed)
    (CallFunction|SetRandomRate))
  (for (_array_element _array_index) (Variables|Default|GetDoorComponents)
    (bind _asanimated_cube (Utilities|Casting|CastToAnimatedCube (Variables|/Script/Engine.ChildActorComponent|GetChildActor _array_element)))
    (Components|Timeline|SetPlayRate (Variables|/Game/Blueprints/AnimatedCube.AnimatedCube_C|GetMoveTimeline _asanimated_cube) (Utilities|Array|Get(acopy) (Variables|Default|GetDoorPlayRates) _array_index))
    (Class|Switchable|SwitchSignal(Message) _asanimated_cube SignalOnOff)))

(fn ConstructionScript
  (Variables|Default|SetDoorComponents (Actor|GetComponentsByClass "/Script/Engine.ChildActorComponent"))
  (if (Variables|Default|GetRandomSpeed)
    (CallFunction|SetRandomRate)
    (else
      (Variables|Default|SetDoorPlayRates (Utilities|Array|MakeArray 0.4 1.2 0.8 0.8 1.0 0.6)))))

(fn SetRandomRate
  (bind _output_get (Variables|Default|SetDoorPlayRates (Utilities|Array|MakeArray (Math|Random|RandomFloat) (Math|Random|RandomFloat) (Math|Random|RandomFloat) (Math|Random|RandomFloat) (Math|Random|RandomFloat) (Math|Random|RandomFloat))))
  (for (_array_element _array_index) _output_get
    (Utilities|Array|SetArrayElem (Variables|Default|GetDoorPlayRates) _array_index (Math|Float|Clamp(Float) (* _array_element 2.0) 0.3 2.0))))