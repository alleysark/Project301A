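; AnimatedCube is an actor whose cube slides along its local X axis in response to an on/off switch signal.
; The construction script caches the cube's default relative location and its X half-extent.
; SwitchSignal plays or reverses a timeline, whose curve value feeds Animate to offset the cube by up to its full width, scaled by that curve, without sweeping.
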(event Collision|EventActorBeginOverlap
  (params (OtherActor :type Actor%20Object%20Reference)))

(event EventTick
  (params (DeltaSeconds :type Float%20%28single-precision%29)))

(event EventSwitchSignal
  (params (SignalOnOff :type Boolean))
  (if SignalOnOff
    (bind _cubicbasecurve (Timeline|MoveTimeline Play)
      (:Update
        (CallFunction|Animate _cubicbasecurve)))
    (else
      (Timeline|MoveTimeline Reverse))))

(fn ConstructionScript
  (bind _cube (Variables|Default|GetCube))
  (Variables|Default|SetCubeDefaultLocation (Variables|/Script/Engine.SceneComponent|GetRelativeLocation _cube))
  (Variables|Default|SetCubeSizeX (.X (Math|Vector|BreakVector (.BoxExtent (Collision|GetComponentBounds _cube))))))

(fn Animate
  (params (TimeLineValue :type Float%20%28single-precision%29))
  (Transformation|SetRelativeLocation (Variables|Default|GetCube) (+ (Math|Vector|MakeVector (* 2.0 TimeLineValue (Variables|Default|GetCubeSizeX)) 0.0 0.0) (Variables|Default|GetCubeDefaultLocation)) false))