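; BP_Gear_Box is a gear box actor that continuously spins two groups of components in opposite directions.
; The construction script caches the direct children of the ClockWiseComponents and CounterClockwiseComponents parents into two arrays.
; Tick applies local yaw to each cached component at RotationVelocity scaled by delta time, negated for the counter-clockwise group, so a component's parent alone sets its spin direction.
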(event EventBeginPlay)

(event Collision|EventActorBeginOverlap
  (params (OtherActor :type Actor%20Object%20Reference)))

(event EventTick
  (params (DeltaSeconds :type Float%20%28single-precision%29))
  (bind _rotationvelocity (Variables|Default|GetRotationVelocity))
  (bind _returnvalue (* DeltaSeconds _rotationvelocity))
  (bind _returnvalue_2 (Class|KismetMathLibrary|MakeRot 0.0 _returnvalue 0.0))
  (Utilities|FlowControl|Sequence
    (:then_0
      (for _array_element (Variables|Default|GetArray_CW)
        (Transformation|AddLocalRotation _array_element _returnvalue_2 false)))
    (:then_1
      (for _array_element_2 (Variables|Default|GetArray_CCW)
        (Transformation|AddLocalRotation _array_element_2 (* _returnvalue_2 -1.0) false)))))

(fn ConstructionScript
  (Variables|Default|SetArray_CW (Components|GetChildrenComponents (Variables|Default|GetClockWiseComponents) false))
  (Variables|Default|SetArray_CCW (Components|GetChildrenComponents (Variables|Default|GetCounterClockwiseComponents) false)))