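; BP_SwitchableStair_renew is a circuit-switchable staircase whose steps move between start and end points when power is supplied, and back when it is cut.
; Tick plays or reverses the Moving timeline from PowerSupplied, and its updates lerp each step's relative location.
; The construction script adds or destroys step meshes toward NumSteps, calls UpdateStair and sets the timeline rate from AnimationTime.
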(event EventTick
  (params (DeltaSeconds :type Float%20%28single-precision%29))
  (if (Variables|Default|GetPowerSupplied)
    (bind _alpha (Timeline|Moving Play)
      (:Update
        (for _index (range 0 (- (Variables|Default|GetNumSteps) 1))
          (Transformation|SetRelativeLocation (Utilities|Array|Get(acopy) (Variables|Default|GetCurSteps) (+ _index 1)) (Math|Vector|Lerp(Vector) (Utilities|Array|Get(acopy) (Variables|Default|GetStepStartPoints) _index) (Utilities|Array|Get(acopy) (Variables|Default|GetStepEndPoints) _index) _alpha) false))))
    (else
      (Timeline|Moving Reverse))))

(event EventBeginPlay)

(event Collision|EventActorBeginOverlap
  (params (OtherActor :type Actor%20Object%20Reference)))

(fn ConstructionScript
  (CallFunction|ConstructStair)
  (Class|SwitchableStairRenew|UpdateStair)
  (Components|Timeline|SetPlayRate (Variables|Default|GetMoving) (/ 1.0 (Variables|Default|GetAnimationTime))))

(fn ConstructStair
  (bind _numsteps (Variables|Default|GetNumSteps))
  (bind _numsteps_2 (Variables|Default|GetNumSteps))
  (bind _output_get (Variables|Default|SetCurSteps (Components|GetChildrenComponents (Variables|Default|GetRootPosition) false)))
  (if (< (Utilities|Array|Length _output_get) _numsteps)
    (for _index (range (Utilities|Array|Length _output_get) _numsteps_2)
      (bind _returnvalue (AddComponent|AddStaticMeshComponent false))
      (Utilities|Array|Add (Variables|Default|GetCurSteps) _returnvalue))
    (elif (> (Utilities|Array|Length _output_get) _numsteps)
      (for _index_2 (range _numsteps_2 (Utilities|Array|Length _output_get))
        (Components|DestroyComponent (Utilities|Array|Get(acopy) (Variables|Default|GetCurSteps) _index_2))))))